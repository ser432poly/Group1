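; HUD Blueprint that draws a "Welcome!" message on screen.
; DrawHUD passes through a gate that the ShowText event opens or closes with a boolean to toggle the message.
; A CountdownTimer function draws a zero-padded minutes:seconds clock, and two timelines compute countdown and count-up values.
; All of that timer logic is disconnected: BeginPlay is empty and nothing runs the timelines or calls CountdownTimer.
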(event EventDrawHUD
  (params (SizeX :type Integer) (SizeY :type Integer))
  ;[1 1 1] Write "Welcome" text
  (Utilities|FlowControl|Gate true
    (:Exit
      (HUD|DrawText "Welcome!" "(R=0.059861,G=0.800000,B=0.054797,A=1.000000)" 4.5e+02 0.0 "/Game/Blueprints/HUD/NewFont.NewFont" 1.0 true))))

(event EventBeginPlay
  ;[1 1 1] Timer
)

(event EventShowText
  (params (Show%20Text? :type Boolean))
  ;[1 1 1] Write "Welcome" text
  (if Show%20Text?
    (Utilities|FlowControl|Gate true) ; enters at Open
    (else
      (Utilities|FlowControl|Gate true) ; enters at Close
    )))

(fn ConstructionScript)

(fn CountdownTimer
  (if (> (Variables|Default|GetHUD_Time_Second) 9)
    (HUD|DrawText (Utilities|String|Append (Utilities|String|Append (Utilities|String|ToString(Integer) (Variables|Default|GetHUD_Time_Minute)) ":") (Utilities|String|ToString(Integer) (Variables|Default|GetHUD_Time_Second))) "(R=1.000000,G=1.000000,B=1.000000,A=1.000000)" 1e+03 2e+01 "/Game/Blueprints/HUD/NewFont.NewFont" 1.0 false)
    (else
      (HUD|DrawText (Utilities|String|Append (Utilities|String|Append (Utilities|String|ToString(Integer) (Variables|Default|GetHUD_Time_Minute)) ":0") (Utilities|String|ToString(Integer) (Variables|Default|GetHUD_Time_Second))) "(R=1.000000,G=1.000000,B=1.000000,A=1.000000)" 1e+03 2e+01 "/Game/Blueprints/HUD/NewFont.NewFont" 1.0 false))))